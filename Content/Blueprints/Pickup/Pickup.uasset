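; Pickup actor for health or ammo items that players collect and that respawns after a delay.
; The construction script picks the item mesh from the Type setting.
; Use notifies the character with the type, then hides the mesh and flags it as taken.
; Tick counts up a timer while taken and shows the item again once RespawnTime passes, with CanPickUp exposing availability.
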(event Custom|Pickup
  ;[1 1 1] Pickup
  (Rendering|SetVisibility (Variables|Default|GetItem) false false)
  (Variables|Default|SetTimer 0.0)
  (Variables|Default|SetHasBeenPickedUp true))

(event Custom|Respawn
  ;[1 1 1] Respawn
  (Rendering|SetVisibility (Variables|Default|GetItem) true false)
  (Variables|Default|SetHasBeenPickedUp false))

(event EventBeginPlay)

(event Collision|EventActorBeginOverlap
  (params (OtherActor :type Actor%20Object%20Reference)))

(event EventTick
  (params (DeltaSeconds :type Float%20%28single-precision%29))
  (if (Variables|Default|GetHasBeenPickedUp)
    (bind _output_get (Variables|Default|SetTimer (+ DeltaSeconds (Variables|Default|GetTimer))))
    (if (> _output_get (Variables|pick|GetRespawnTime))
      (CallFunction|Respawn))))

(event EventUse
  (params (Controller :type Controller%20Object%20Reference) (Character :type Pawn%20Object%20Reference))
  ;[1 1 1] PickupEvent
  (if (not (Variables|Default|GetHasBeenPickedUp))
    (Class|PawnInterFace|Pickedup(Message) Character (Variables|pick|GetType))
    (CallFunction|Pickup)))

(fn ConstructionScript
  (bind _itemmeshes (Variables|pick|GetItemMeshes))
  (Components|StaticMesh|SetStaticMesh (Variables|Default|GetItem) (Utilities|Select :Index (Variables|pick|GetType) :NewEnumerator0 (Utilities|Array|Get(acopy) _itemmeshes) :NewEnumerator1 (Utilities|Array|Get(acopy) _itemmeshes 1))))

(fn CanPickUp
  (return (not (Variables|Default|GetHasBeenPickedUp))))