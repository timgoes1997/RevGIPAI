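; TPBase is a base shooter pawn with a socketed gun, health, ammo and pickup handling.
; FireGun spends clip rounds on a line trace that applies random-range damage, while Reload refills the clip from reserve ammo.
; Damage either passes the instigator's transform to a damage event or, below one health, asks the GameMode to spawn and destroys the pawn.
; Item pickup uses a forward multi-trace and interface messages; health and ammo gains are capped.
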(event EventBeginPlay
  (Transformation|AttachComponentToComponent (Variables|Default|GetGun) (Variables|Character|GetMesh) "GunSocket" "SnapToTarget" "SnapToTarget" "SnapToTarget" true))

(event Game|Damage|EventAnyDamage
  (params (Damage :type Float%20%28single-precision%29) (DamageType :type Damage%20Type%20Object%20Reference) (InstigatedBy :type Controller%20Object%20Reference) (DamageCauser :type Actor%20Object%20Reference))
  ;[1 1 1] Damage event
  (bind _output_get (Variables|Default|SetHealth (- (Variables|Default|GetHealth) Damage)))
  (if (< _output_get 1.0)
    (CallFunction|Respawn)
    (else
      (Default|CallDamageEvent (Transformation|GetActorTransform InstigatedBy)))))

(event EventFireGun
  (params (Start :type Vector :default "0, 0, 0") (End :type Vector :default "0, 0, 0"))
  ;[1 1 1] FireGun
  (if (> (Variables|Default|GetCurrentClip) 0)
    (Variables|Default|SetCurrentClip (- (Variables|Default|GetCurrentClip) 1))
    (bind _outhit (Collision|LineTraceByChannel Start End "TraceTypeQuery2" false 0 "ForDuration"))
    (Game|Damage|ApplyDamage (.HitActor (Collision|BreakHitResult _outhit)) (Math|Random|RandomFloatinRange (Variables|Default|GetMinDamage) (Variables|Default|GetMaxDamage)) (Pawn|GetController) self "/Script/Engine.DamageType")
    (else
      (Development|PrintString "No Ammo"))))

(event EventPickedup
  (params (PickupType :type EPickupType%20Enum :default "NewEnumerator0"))
  ;[1 1 1] Pickup Events
  (switch Utilities|FlowControl|Switch|SwitchonEPickupType PickupType
    (:NewEnumerator0
      (CallFunction|Heal))
    (:NewEnumerator1
      (CallFunction|AddAmmo))))

(event EventAddAmmo
  (bind _maxammo (Variables|Default|GetMaxAmmo))
  ;[1 1 1] AddAmmo
  (bind _output_get (Variables|Default|SetAmmo (select (< (+ (Variables|Default|GetAmmo) (Variables|Default|GetAmmoOnPickup)) _maxammo) (+ (Variables|Default|GetAmmo) (Variables|Default|GetAmmoOnPickup)) _maxammo)))
  (Development|PrintString (Utilities|String|ToString(Integer) _output_get)))

(event EventReload
  ;[1 1 1] Reload
  (if (> (Variables|Default|GetAmmo) 0)
    (if (> (- (Variables|Default|GetAmmoInClip) (Variables|Default|GetCurrentClip)) (Variables|Default|GetAmmo))
      (Variables|Default|SetCurrentClip (+ (Variables|Default|GetCurrentClip) (Variables|Default|GetAmmo)))
      (Variables|Default|SetAmmo 0)
      (else
        (Variables|Default|SetAmmo (- (Variables|Default|GetAmmo) (- (Variables|Default|GetAmmoInClip) (Variables|Default|GetCurrentClip))))
        (Variables|Default|SetCurrentClip (Variables|Default|GetAmmoInClip))))
    (Development|PrintString (Utilities|String|Append (Utilities|String|ToString(Integer) (Variables|Default|GetCurrentClip)) "/" (Utilities|String|ToString(Integer) (Variables|Default|GetAmmo))))))

(event EventHeal
  (bind _maxhealth (Variables|Default|GetMaxHealth))
  ;[1 1 1] Heal pawn
  (bind _output_get (Variables|Default|SetHealth (select (< (+ (Variables|Default|GetHealth) (Variables|Default|GetHealOnPickup)) _maxhealth) (+ (Variables|Default|GetHealth) (Variables|Default|GetHealOnPickup)) _maxhealth)))
  (Development|PrintString (Utilities|String|ToString(Float) _output_get)))

(event EventPickupItem
  (bind (_start _end) (Utilities|GetForwardLineTrace))
  ;[1 1 1] Event for pickingup items
  (bind _outhits (Collision|MultiLineTraceByChannel _start _end "TraceTypeQuery1" false 0 "None"))
  (for _array_element _outhits
    (if (Utilities|DoesObjectImplementInterface (.hitactor _array_element) "/Game/Blueprints/Pickup/PickupInterface.PickupInterface_C")
      (bind _canpickup (Class|PickupInterface|CanPickUp(Message) (.hitactor _array_element)))
      (if _canpickup
        (Class|PickupInterface|Use(Message) (.hitactor _array_element) (Pawn|GetController) self)))))

(fn ConstructionScript
  (Transformation|AttachComponentToComponent (Variables|Default|GetGun) (Variables|Character|GetMesh) "GunSocket" "SnapToTarget" "SnapToTarget" "SnapToTarget" true))

(fn Respawn
  (Class|IGameMode|Spawn(Message) (Game|GetGameMode) (Pawn|GetController) self)
  (Class|Pawn|DetachfromControllerPendingDestroy)
  (Actor|DestroyActor))

(fn GetMuzzleLocation
  (return (Transformation|GetSocketLocation (Variables|Default|GetGun) "Muzzle")))